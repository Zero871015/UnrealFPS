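; Soldier Blueprint that automatically fires a weapon in intermittent bursts and reloads when empty.
; Tick runs a Delay with a random interval from the FireRate range, then a FlipFlop toggles IsFiring on and off.
; On each firing phase it calls Fire on the weapon and triggers Reload when the result is zero or less.
; The construction script stores the actor transform as RespawnPoint.
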(event `self.ReceiveTick`
  (params (DeltaSeconds :type "Float (single-precision)"))
  (bind (_x _y) (`KismetMathLibrary.BreakVector2D` (`self.FireRate`)))
  (`KismetSystemLibrary.Delay` (`KismetMathLibrary.RandomFloatInRange` _x _y))
  (`/Engine/EditorBlueprintResources/StandardMacros.FlipFlop`
    (:`A`
      (set `self.IsFiring` true)
      (bind _ammo (`/Game/__ADDONS/T91/T91rifle.Fire` (`self.Weapon`) true))
      (if (<= _ammo 0)
        (`self.Reload`)))
    (:`B`
      (set `self.IsFiring` false))))

(fn `UserConstructionScript`
  (set `self.RespawnPoint` (`self.GetTransform`)))